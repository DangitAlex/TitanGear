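; BP_RespawnPoint is a placed actor that returns the player to its transform when Backspace is pressed.
; It enables input on BeginPlay, then on the key teleports the character, zeroes movement velocity and aligns control rotation.
; It also calls CableRetrieveAll on the character's child-actor BP_Titan_Gear to pull back all cables.
; In the construction script, a SnapToPlayerSpawn toggle acts as an editor button that moves it onto the first PlayerStart.
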(event `self.ReceiveBeginPlay`
  (`self.EnableInput` (`GameplayStatics.GetPlayerController` 0)))

(event `Key|BackSpace`
  (params (Key :type "Key Structure" :default "AnyKey"))
  (bind _returnvalue (`GameplayStatics.GetPlayerCharacter` 0))
  (bind _returnvalue_2 (`self.GetTransform`))
  (:`Pressed`
    (`self.K2_SetActorTransform` _returnvalue _returnvalue_2 false false)
    (set `MovementComponent.Velocity` (0.0 0.0 0.0) (`KismetArrayLibrary.Array_Get` (`self.K2_GetComponentsByClass` _returnvalue "/Script/Engine.CharacterMovementComponent")))
    (bind _asbp_titan_gear (cast `/Game/_CreatedAssets/Blueprints/Player/BP_Titan_Gear` (`ChildActorComponent.ChildActor` (`KismetArrayLibrary.Array_Get` (`self.K2_GetComponentsByClass` _returnvalue "/Script/Engine.ChildActorComponent")))))
    (`/Game/_CreatedAssets/Blueprints/Player/BP_Titan_Gear.Cable_Retrieve_All` _asbp_titan_gear)
    (`Controller.SetControlRotation` (`GameplayStatics.GetPlayerController` 0) (.rotation _returnvalue_2))))

(fn `UserConstructionScript`
  (if (`self.snapToPlayerSpawn`)
    (set `self.snapToPlayerSpawn` false)
    (bind _outactors (`GameplayStatics.GetAllActorsOfClass` "/Script/Engine.PlayerStart"))
    (bind _item (`KismetArrayLibrary.Array_Get` _outactors))
    (`self.K2_SetActorLocationAndRotation` (`self.K2_GetActorLocation` _item) (`self.K2_GetActorRotation` _item))))