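; Actor component that sets up the player's Titan gear on its owning pawn and exposes its wall-running state.
; On BeginPlay it finds the BP_Titan_Gear spawned through one of the pawn's child actor components and caches it.
; It creates the Titan HUD widget, links it to the gear, then connects the gear to the player controller and that widget.
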(event EventBeginPlay
  (CallFunction|InitializeReferences))

(fn InitializeReferences
  (bind _aspawn (Utilities|Casting|CastToPawn (Components|GetOwner)))
  (Variables|Default|SetRef_OwningPawn _aspawn)
  (bind _array_element (Utilities|Array|ForEachLoopwithBreak (Actor|GetComponentsByClass _aspawn "/Script/Engine.ChildActorComponent") :!label _label)
    (:LoopBody
      (bind _asbp_titan_gear (Utilities|Casting|CastToBP_Titan_Gear (Variables|/Script/Engine.ChildActorComponent|GetChildActor _array_element)))
      (Variables|Default|SetRef_TitanGear _asbp_titan_gear)
      (goto _label Break))
    (:Completed
      (bind _widgetref (CallFunction|InitializeHUD))
      (bind _returnvalue (Utilities|Casting|CastToPlayerController (Pawn|GetController _aspawn)))
      (Default|ConnectGear (Variables|Default|GetRef_TitanGear) _returnvalue _widgetref))))

(fn InitializeHUD
  (bind _returnvalue (Utilities|Casting|CastToPlayerController (Pawn|GetController (Variables|Default|GetRef_OwningPawn))))
  (bind _returnvalue_2 (UserInterface|CreateWidget "/Game/_CreatedAssets/Blueprints/HUD/BP_Titan_HUDWidget.BP_Titan_HUDWidget_C" _returnvalue))
  (UserInterface|Viewport|AddtoViewport _returnvalue_2 0)
  (Default|SetTitanGearRef _returnvalue_2 (Variables|Default|GetRef_TitanGear))
  (return _returnvalue_2))

(fn IsPlayerWallRunning?
  (bind _ref_titangear (Variables|Default|GetRef_TitanGear))
  (Utilities|IsValid _ref_titangear
    (:Is%20Valid
      (LocalVariables|SetwallRunning? (Variables|/Game/_CreatedAssets/Blueprints/Player/BP_Titan_Gear.BP_Titan_Gear_C|GetbIsWallRunning _ref_titangear)))
    (:Is%20Not%20Valid
      (LocalVariables|SetwallRunning? false)))
  (return (LocalVariables|GetwallRunning?)))