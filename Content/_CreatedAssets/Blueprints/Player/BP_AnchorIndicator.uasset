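; Player anchor indicator actor that marks a candidate or committed anchor point with a state-colored mesh.
; UpdateAnchor shows, hides and moves it, while SetAnchorState swaps materials between check, check-center and anchor.
; Reaching the anchor state sets LockState, which blocks further state, visibility and position updates through these functions.
; A stored skeletal mesh component and bone name let it attach at its world position to follow that bone, or detach.
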(fn `AnchorToAvailableSK`
  (params (`detach?` :type Boolean))
  (if `detach?`
    (if (`self.isAnchoredToSK?`)
      (`self.DetachRootComponentFromParent` true)
      (set `self.isAnchoredToSK?` false)
      (set `self.Ref_AnchoredSK` null)
      (set `self.AnchoredSK_BoneName` "None"))
    (elif (`self.isSKAvailable?`)
      (`self.K2_AttachRootComponentTo` (`self.Ref_AnchoredSK`) (`self.AnchoredSK_BoneName`) "KeepWorldPosition")
      (set `self.isAnchoredToSK?` true))))

(fn `SetAnchorState`
  (params (newState :type "/Game/_CreatedAssets/Blueprints/Player/E_AnchorState Enum"))
  (bind _indicatormesh (`self.IndicatorMesh`))
  (if (not (`self.lockState?`))
    (bind _output_get (set `self.currentAnchorState` newState))
    (switch `/Game/_CreatedAssets/Blueprints/Player/E_AnchorState` _output_get
      (:`NewEnumerator1`
        (`PrimitiveComponent.SetMaterial` _indicatormesh 0 "/Game/_CreatedAssets/Materials/M_Indicator_Check.M_Indicator_Check"))
      (:`NewEnumerator2`
        (`PrimitiveComponent.SetMaterial` _indicatormesh 0 "/Game/_CreatedAssets/Materials/M_Indicator_Check_Center.M_Indicator_Check_Center"))
      (:`NewEnumerator0`
        (`PrimitiveComponent.SetMaterial` _indicatormesh 0 "/Game/_CreatedAssets/Materials/M_Indicator_Anchor.M_Indicator_Anchor")
        (set `self.lockState?` true)))))

(fn `SetHiddenState`
  (params (`hidden?` :type Boolean))
  (bind _defaultsceneroot (`self.DefaultSceneRoot`))
  (if (`self.lockState?`)
    _
    (elif (!= `hidden?` (`self.isHidden?`))
      (bind _output_get (set `self.isHidden?` `hidden?`))
      (if _output_get
        (`self.SetAnchorState` "NewEnumerator1")
        (`SceneComponent.SetVisibility` _defaultsceneroot false true)
        (else
          (`SceneComponent.SetVisibility` _defaultsceneroot true true))))))

(fn `SetSKReference`
  (params (SKHit :type "/Game/_CreatedAssets/Blueprints/Player/SK_Hit Structure"))
  (bind (_sk_component_ref _bonename) (break `/Game/_CreatedAssets/Blueprints/Player/SK_Hit` SKHit))
  (`/Engine/EditorBlueprintResources/StandardMacros.IsValid` _sk_component_ref
    (:`Is Valid`
      (set `self.Ref_AnchoredSK` _sk_component_ref)
      (set `self.AnchoredSK_BoneName` _bonename)
      (set `self.isSKAvailable?` true))
    (:`Is Not Valid`
      (set `self.isSKAvailable?` false))))

(fn `UpdateAnchor`
  (params (`manualHide?` :type Boolean) (`anchorAvailable?` :type Boolean) (newLocation :type "Vector Structure") (newState :type "/Game/_CreatedAssets/Blueprints/Player/E_AnchorState Enum"))
  (if (`self.lockState?`)
    _
    (elif `manualHide?`
      (`self.SetHiddenState` true)
      (elif `anchorAvailable?`
        (`self.SetHiddenState` false)
        (`self.K2_SetActorLocation` newLocation false true)
        (`self.SetAnchorState` newState)
        (else
          (`self.SetHiddenState` true))))))

(fn `UserConstructionScript`)