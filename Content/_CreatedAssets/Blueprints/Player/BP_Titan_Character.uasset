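; BP_Titan_Character is a player character Blueprint carrying a TitanGear child actor and a BPTitanGearComponent.
; Both BeginPlay and the construction script call InitializePlayerReferences, passing the gear actor and component, character movement, camera, camera boom and the mesh's anim instance.
; It holds only this reference wiring, with no movement or gear logic in its graphs.
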(event `self.ReceiveBeginPlay`
  (`/Game/_CreatedAssets/Blueprints/Player/BP_TitanGear_Functions.InitializePlayerReferences` (`self.TitanGear`) (`self.CharacterMovement`) (`self.Camera`) (`self.CameraBoom`) (`self.BP_Titan_GearComponent`) (`SkeletalMeshComponent.GetAnimInstance` (`self.Mesh`))))

(fn `UserConstructionScript`
  (`/Game/_CreatedAssets/Blueprints/Player/BP_TitanGear_Functions.InitializePlayerReferences` (`self.TitanGear`) (`self.CharacterMovement`) (`self.Camera`) (`self.CameraBoom`) (`self.BP_Titan_GearComponent`) (`SkeletalMeshComponent.GetAnimInstance` (`self.Mesh`))))