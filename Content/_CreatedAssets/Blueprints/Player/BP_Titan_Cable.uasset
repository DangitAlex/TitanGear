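; One grappling cable, left or right, of the player's Titan gear, fired at an anchor indicator and retrieved.
; A Tick-driven state machine (docked, firing, anchored, retrieving) interpolates length during fire and retrieval, notifying the gear of state changes.
; The cable mesh follows the gear's start point, rotates toward the anchor and Z-scales to length, hiding when docked.
; Distance over set length yields the tension ratio behind the taut check.
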(event EventTick
  (params (DeltaSeconds :type Float%20%28single-precision%29))
  (bind _ref_titangear (Variables|TitanGear|GetRef_TitanGear))
  (if (Utilities|Enum|NotEqual(Enum) (Variables|GrappleSystem|GetcurrentFireState) "NewEnumerator4")
    (Cable_Update|UpdateCableStartandEndPoints)
    (Cable_Update|RotatetoAnchor))
  (if (Get|HasatLeastFired?)
    (Cable_Update|UpdateDistancetoAnchor))
  (switch Utilities|FlowControl|Switch|SwitchonE_CableFireState (Variables|GrappleSystem|GetcurrentFireState)
    (:NewEnumerator4
      _)
    (:NewEnumerator0
      (Utilities|InterpCableLength (Math|Vector|VectorLength (- (Variables|GrappleSystem|GetanchorLocation) (Variables|GrappleSystem|GetFireStartVector))) (Variables|GrappleSystem|GetcableSpeed_Fire)
        (:REACHED
          (Variables|GrappleSystem|SetcurrentFireState "NewEnumerator1")
          (Variables|GrappleSystem|SetcurrentLength (Variables|GrappleSystem|GetdistanceFromRootToAnchor))
          (Default|RefreshAnchoredCableVariable _ref_titangear))
        (:NOT_YET
          _)))
    (:NewEnumerator1
      (Cable_Update|UpdateCableMeshLength (Variables|GrappleSystem|GetdistanceFromRootToAnchor)))
    (:NewEnumerator2
      (bind _output_get (Variables|GrappleSystem|SetdistanceFromRootToAnchor 0.0))
      (Utilities|InterpCableLength _output_get (Variables|GrappleSystem|GetcableSpeed_Retrieve)
        (:REACHED
          (Variables|GrappleSystem|SetcurrentFireState "NewEnumerator4")
          (Variables|GrappleSystem|SetcurrentLength 0.0)
          (Default|RefreshAnchoredCableVariable _ref_titangear))
        (:NOT_YET
          _))))
  (Cable_Update|UpdateCableVisibility))

(fn ConstructionScript
  (Cable_Update|UpdateCableMeshLength (Variables|GrappleSystem|GetcurrentLength)))

(fn RotatetoAnchor
  (Transformation|SetWorldRotation (Variables|Default|GetCableMesh) (Math|Rotator|MakeRotfromZ (Class|KismetMathLibrary|GetDirectionVector (Transformation|GetWorldLocation (Variables|Default|GetCableRoot)) (Variables|GrappleSystem|GetanchorLocation))) false true))

(fn Fire
  (params (IndicatorRef :type BP%20Anchor%20Indicator%20Object%20Reference))
  (bind _ref_cablestart (Variables|Default|GetRef_CableStart))
  (bind _returnvalue (Transformation|GetWorldLocation _ref_cablestart))
  (bind _output_get (Variables|GrappleSystem|SetRef_AnchorIndicator IndicatorRef))
  (bind _output_get_2 (Variables|GrappleSystem|SetanchorLocation (Transformation|GetActorLocation _output_get)))
  (Variables|GrappleSystem|SetFireStartVector _returnvalue)
  (Variables|GrappleSystem|SetcurrentFireState "NewEnumerator0")
  (Variables|GrappleSystem|SetdistanceFromRootToAnchor (Math|Vector|VectorLength (- _output_get_2 _returnvalue)))
  (Default|RefreshAnchoredCableVariable (Variables|TitanGear|GetRef_TitanGear)))

(fn UpdateCableMeshLength
  (params (newCableLength :type Float%20%28single-precision%29))
  (bind _ref_titangear (Variables|TitanGear|GetRef_TitanGear))
  (bind _cablewidth (Variables|Cable|GetcableWidth))
  (bind _returnvalue (/ _cablewidth 1e+02))
  (Utilities|IsValid _ref_titangear
    (:Is%20Valid
      (LocalVariables|SetmaxRange (Variables|/Game/_CreatedAssets/Blueprints/Player/BP_Titan_Gear.BP_Titan_Gear_C|Getgear_cableLength_MAX _ref_titangear)))
    (:Is%20Not%20Valid
      (LocalVariables|SetmaxRange 1.5e+04)))
  (bind _output_get (Variables|GrappleSystem|SetcurrentMeshLength newCableLength))
  (LocalVariables|SetnewScale (Math|Vector|MakeVector _returnvalue _returnvalue (Math|Float|Clamp(Float) (/ _output_get 1e+02) 0.0001 (LocalVariables|GetmaxRange))))
  (Transformation|SetRelativeScale3D (Variables|Default|GetCableMesh) (LocalVariables|GetnewScale)))

(fn UpdateDistancetoAnchor
  (bind _cableroot (Variables|Default|GetCableRoot))
  (bind _anchorlocation (Variables|GrappleSystem|GetanchorLocation))
  (bind _returnvalue (Transformation|GetWorldLocation _cableroot))
  (bind _returnvalue_2 (- _anchorlocation _returnvalue))
  (Variables|GrappleSystem|SetdistanceFromRootToAnchor (Math|Vector|VectorLength _returnvalue_2))
  (Variables|GrappleSystem|SetvectorToAnchor (Math|Vector|Normalize _returnvalue_2))
  (Variables|GrappleSystem|SetcableTensionRatio (/ (Variables|GrappleSystem|GetdistanceFromRootToAnchor) (Variables|GrappleSystem|GetcurrentLength))))

(fn InitializeCable
  (params (side :type E_CableSide%20Enum) (GearRef :type BP%20Titan%20Gear%20Object%20Reference))
  (bind _output_get (Variables|Cable|SetcableSide side))
  (bind _output_get_2 (Variables|TitanGear|SetRef_TitanGear GearRef))
  (switch Utilities|FlowControl|Switch|SwitchonE_CableSide _output_get
    (:NewEnumerator0
      (Variables|Default|SetRef_CableStart (Variables|/Game/_CreatedAssets/Blueprints/Player/BP_Titan_Gear.BP_Titan_Gear_C|GetCableStart_Left _output_get_2)))
    (:NewEnumerator1
      (Variables|Default|SetRef_CableStart (Variables|/Game/_CreatedAssets/Blueprints/Player/BP_Titan_Gear.BP_Titan_Gear_C|GetCableStart_Right _output_get_2)))))

(fn Retrieve
  (Variables|GrappleSystem|SetcurrentFireState "NewEnumerator2")
  (Default|AnchortoAvailableSK (Variables|GrappleSystem|GetRef_AnchorIndicator) true)
  (Variables|/Game/_CreatedAssets/Blueprints/Player/BP_AnchorIndicator.BP_AnchorIndicator_C|SetlockState? (Variables|GrappleSystem|GetRef_AnchorIndicator) false)
  (Variables|GrappleSystem|SetRef_AnchorIndicator 0)
  (Default|RefreshAnchoredCableVariable (Variables|TitanGear|GetRef_TitanGear)))

(fn UpdateCableStartandEndPoints
  (bind _ref_anchorindicator (Variables|GrappleSystem|GetRef_AnchorIndicator))
  (Transformation|SetWorldLocation (Variables|Default|GetCableRoot) (Transformation|GetWorldLocation (Variables|Default|GetRef_CableStart)) false true)
  (Utilities|IsValid _ref_anchorindicator
    (:Is%20Valid
      (Variables|GrappleSystem|SetanchorLocation (Transformation|GetActorLocation _ref_anchorindicator)))))

(fn UpdateCableVisibility
  (bind _cablemesh (Variables|Default|GetCableMesh))
  (if (Utilities|Enum|Equal(Enum) (Variables|GrappleSystem|GetcurrentFireState) "NewEnumerator4")
    (Rendering|SetVisibility _cablemesh false false)
    (else
      (Rendering|SetVisibility _cablemesh true false))))

(fn IsAnchored?
  (return (Utilities|Enum|Equal(Enum) (Variables|GrappleSystem|GetcurrentFireState) "NewEnumerator1")))

(fn HasatLeastFired?
  (bind _currentfirestate (Variables|GrappleSystem|GetcurrentFireState))
  (return (or (Utilities|Enum|Equal(Enum) _currentfirestate "NewEnumerator1") (Utilities|Enum|Equal(Enum) _currentfirestate "NewEnumerator0"))))

(fn SetLengthtoDistancefromAnchor)

(fn SetLength
  (params (newLength :type Float%20%28single-precision%29))
  (bind _output_get (Variables|GrappleSystem|SetcurrentLength newLength))
  (Cable_Update|UpdateCableMeshLength _output_get))

(fn CanbeRetrieved?
  (return (Utilities|Enum|NotEqual(Enum) (Variables|GrappleSystem|GetcurrentFireState) "NewEnumerator4")))

(fn IsTaut?
  (return (and (>= (Variables|GrappleSystem|GetcableTensionRatio) 1.0) (Get|IsAnchored?))))

(fn GetOffsetfromPlayertoCableStart
  (return (- (Transformation|GetWorldLocation (Variables|/Game/_CreatedAssets/Blueprints/Player/BP_Titan_Gear.BP_Titan_Gear_C|GetRef_PlayerPhysicsRoot (Variables|TitanGear|GetRef_TitanGear))) (Transformation|GetWorldLocation (Variables|Default|GetRef_CableStart)))))

(fn CanbeFired?
  (return (Utilities|Enum|Equal(Enum) (Variables|GrappleSystem|GetcurrentFireState) "NewEnumerator4")))