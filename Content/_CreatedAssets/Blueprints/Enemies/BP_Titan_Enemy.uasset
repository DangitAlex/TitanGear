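; BP_Titan_Enemy is a Titan enemy that dies when a character carrying a BP_Titan_GearComponent overlaps its weak point.
; Kill flags it dead, switches the skeletal mesh to physics ragdoll and activates a death particle.
; The construction script applies animation rate, titan scale and weak point scale.
; A self-resetting SnapToFloorNOW bool acts as an editor button, using a downward line trace to move the root onto the floor.
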(event `self.WeakPoint.OnComponentBeginOverlap`
  (params (OtherActor :type "Actor Object Reference") (OtherComp :type "PrimitiveComponent Object Reference") (OtherBodyIndex :type Integer) (bFromSweep :type Boolean) (SweepResult :type "HitResult Structure (by ref)"))
  (bind _ascharacter (cast `Character` OtherActor))
  (if (> (`KismetArrayLibrary.Array_Length` (`self.K2_GetComponentsByClass` _ascharacter "/Game/_CreatedAssets/Blueprints/Player/BP_Titan_GearComponent.BP_Titan_GearComponent_C")) 0)
    (if (not (`self.isDead?`))
      (`self.Kill`))))

(fn `Kill`
  (bind _skeletalmesh (`self.SkeletalMesh`))
  (set `self.isDead?` true)
  (`SkeletalMeshComponent.SetAllBodiesSimulatePhysics` _skeletalmesh true)
  (`PrimitiveComponent.WakeAllRigidBodies` _skeletalmesh)
  (`ActorComponent.Activate` (`self.DeathParticle`) true))

(fn `SnapToFloor`
  (bind (_outhit _returnvalue) (`KismetSystemLibrary.LineTraceSingle` (`SceneComponent.K2_GetComponentLocation` (`self.SkeletalMesh`)) (* (* (`KismetMathLibrary.GetUpVector` (`self.K2_GetActorRotation`)) -1) 100000.0) "TraceTypeQuery1"))
  (if _returnvalue
    (`SceneComponent.K2_SetWorldLocation` (`self.DefaultSceneRoot`) (`.ImpactPoint` (`GameplayStatics.BreakHitResult` _outhit)) false true)))

(fn `UserConstructionScript`
  (set `SkeletalMeshComponent.GlobalAnimRateScale` (`self.animScale`) (`self.SkeletalMesh`))
  (`SceneComponent.SetWorldScale3D` (`self.SkeletalMesh`) (`KismetMathLibrary.Conv_DoubleToVector` (* (`self.TitanScale`) 5.0)))
  (`|ExecutionSequence`
    (:`then_0`
      (if (`self.snapToFloor_NOW`)
        (set `self.snapToFloor_NOW` false)
        (`self.SnapToFloor`)))
    (:`then_1`
      (`SceneComponent.SetRelativeScale3D` (`self.WeakPoint`) (`KismetMathLibrary.Conv_DoubleToVector` (`self.weakPointScale`))))))